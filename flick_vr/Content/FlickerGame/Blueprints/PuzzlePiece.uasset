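; A draggable puzzle piece actor that the player picks up by hovering the cursor over it and holding the left mouse button.
; Each tick it sets the attached state from hover and the player's button flag, toggling physics simulation off while held.
; While attached, a line trace from the deprojected mouse position drives a swept move, using the hit location multiplied by a Z-only vector.
; The construction script tints the mesh through a dynamic material's Color parameter.
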(event Custom|CheckAttach
  (if (and (Variables|Default|GetCursor%20Hover) (Variables|/Game/FirstPersonBP/Blueprints/FirstPersonCharacter.FirstPersonCharacter_C|GetLmbDown (Variables|Default|GetPlayer)))
    (CallFunction|SetAttached true)
    (else
      (CallFunction|SetAttached false))))

(event Custom|PickUpMesh
  (bind _returnvalue (Game|GetPlayerController 0))
  (bind (_worldlocation _worlddirection) (Game|Player|ConvertMouseLocationToWorldSpace _returnvalue))
  (if (Variables|Default|GetAttachedToCursor)
    (bind (_outhit _returnvalue_2) (Collision|LineTraceByChannel _worldlocation (* _worldlocation (* _worlddirection (Variables|Default|GetCursorTraceDistance))) "TraceTypeQuery3" false 0 "None"))
    (if _returnvalue_2
      (Transformation|SetActorLocation (* (.Location (Collision|BreakHitResult _outhit)) "0, 0,30.000000") true false))))

(event EventBeginPlay
  ;[1 1 1] GetPlayerReference
  (bind _asfirst_person_character (Utilities|Casting|CastToFirstPersonCharacter (Pawn|GetControlledPawn (Game|GetPlayerController 0))))
  (Variables|Default|SetPlayer _asfirst_person_character))

(event MouseInput|EventActorEndCursorOver
  (Variables|Default|SetCursor%20Hover false))

(event EventTick
  (params (DeltaSeconds :type Float%20%28single-precision%29))
  (CallFunction|CheckAttach)
  (CallFunction|PickUpMesh))

(event MouseInput|EventActorBeginCursorOver
  (Variables|Default|SetCursor%20Hover true))

(fn ConstructionScript
  (bind _piece (Variables|Default|GetPiece))
  (bind _returnvalue (Rendering|Material|CreateDynamicMaterialInstance _piece 0 0 :!class /Script/Engine.PrimitiveComponent))
  (Rendering|Material|SetVectorParameterValue _returnvalue "Color" (Variables|Default|GetColor) :!class /Script/Engine.MaterialInstanceDynamic)
  (Rendering|Material|SetMaterial _piece 0 _returnvalue))

(fn SetAttached
  (params (Attached :type Boolean))
  (Physics|SetSimulatePhysics (Variables|Default|GetPiece) (not Attached))
  (Variables|Default|SetAttachedToCursor Attached))