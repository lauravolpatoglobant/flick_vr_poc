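; SpawnRegion is a Blueprint that spawns units at random points inside its spawn volume box.
; Its SpawnUnit event spawns the given unit class, adjusting position to avoid collisions but always spawning.
; Spawned BaseUnitBP units then receive a default controller, a uniform SpawnScale and the region's Team.
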(event Custom|SpawnUnit
  (params (UnitType :type Actor%20Class%20Reference))
  (bind _spawnscale (Variables|Default|GetSpawnScale))
  (bind _spawnvolume (Variables|Default|GetSpawnVolume))
  (bind _returnvalue (Game|SpawnActorfromClass UnitType (Math|Conversions|ToTransform(Vector) (Math|Random|RandomPointinBoundingBox (Transformation|GetWorldLocation _spawnvolume) (Components|Box|GetScaledBoxExtent _spawnvolume))) "AdjustIfPossibleButAlwaysSpawn" 0 0))
  (bind _asbase_unit_bp (Utilities|Casting|CastToBaseUnitBP _returnvalue))
  (Pawn|SpawnDefaultController _asbase_unit_bp)
  (Transformation|SetActorScale3D _asbase_unit_bp (Math|Vector|MakeVector _spawnscale _spawnscale _spawnscale))
  (Default|SetTeam _asbase_unit_bp (Variables|Default|GetTeam)))

(fn ConstructionScript)