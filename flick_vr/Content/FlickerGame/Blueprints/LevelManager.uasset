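; LevelManager runs the level flow of a battle between player and enemy command bases, from new game to game over.
; BeginPlay caches the terrain, UI screens, spawn regions and base points, identifying regions and points by actor name.
; LoadLevel spawns both bases, grows the terrain and fills a hard-coded, timed unit list per level.
; Tick spawns those units and checks base deaths, then loops to the next level or returns to the title.
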(event EventBeginPlay
  (Utilities|FlowControl|Sequence
    (:then_0
      ;[1 1 1] identifies and stores the terrain actor
      (bind _outactors (Actor|GetAllActorsOfClass "/Game/FlickerGame/Blueprints/Terrain.Terrain_C"))
      (Variables|Default|SetTerrain (Utilities|Array|Get(acopy) _outactors)))
    (:then_1
      ;[1 1 1] identifies and stores the game over message
      (bind _outactors_2 (Actor|GetAllActorsOfClass "/Game/FlickerGame/Blueprints/MessagesDisplay.MessagesDisplay_C"))
      (Variables|Default|SetMessagesDisplay (Utilities|Array|Get(acopy) _outactors_2)))
    (:then_2
      ;[1 1 1] identifies and stores the game title screen
      (bind _outactors_3 (Actor|GetAllActorsOfClass "/Game/FlickerGame/Blueprints/GameTitle.GameTitle_C"))
      (Variables|Default|SetGameTitleScreen (Utilities|Array|Get(acopy) _outactors_3)))
    (:then_3
      ;[1 1 1] identifies and stores the spawn regions
      (bind _outactors_4 (Actor|GetAllActorsOfClass "/Game/FlickerGame/Blueprints/SpawnRegion.SpawnRegion_C"))
      (for _array_element _outactors_4
        (if (Utilities|Enum|Equal(Enum) (Utilities|String|ToString(Object) _array_element) "PlayerSpawnRegion")
          (Variables|Default|SetPlayerSpawnRegion _array_element)
          (else
            (Variables|Default|SetEnemySpawnRegion _array_element)))))
    (:then_4
      ;[1 1 1] identifies and stores the bases spawn points
      (bind _outactors_5 (Actor|GetAllActorsOfClass "/Script/Engine.TargetPoint"))
      (for _array_element_2 _outactors_5
        (if (Utilities|Enum|Equal(Enum) (Utilities|String|ToString(Object) _array_element_2) "PlayerBasePoint")
          (Variables|Default|SetPlayerBaseLocation (Transformation|GetActorLocation _array_element_2))
          (elif (Utilities|Enum|Equal(Enum) (Utilities|String|ToString(Object) _array_element_2) "EnemyBasePoint")
            (Variables|Default|SetEnemyBaseLocation (Transformation|GetActorLocation _array_element_2))))))))

(event EventTick
  (params (DeltaSeconds :type Float%20%28single-precision%29))
  (bind _playerbase (Variables|Default|GetPlayerBase))
  (bind _currentleveldata (Variables|Default|GetCurrentLevelData))
  (bind _enemybase (Variables|Default|GetEnemyBase))
  (bind _levelunitindex (Variables|Default|GetLevelUnitIndex))
  (bind _item (Utilities|Array|Get(acopy) _currentleveldata _levelunitindex))
  (bind (_type _team _spawntime) (Utilities|Struct|BreakUnitData _item))
  (if (Utilities|Enum|Equal(Enum) (Variables|Default|GetState) "NewEnumerator1")
    ;[1 1 1] Check Victory
    (if (Utilities|IsValid _enemybase)
      (if (Variables|/Game/FlickerGame/Blueprints/CommandBase.CommandBase_C|GetIsDead _enemybase)
        ;[1 1 1] show victory screen and advances level
        (Variables|Default|SetState "NewEnumerator2")
        (CallFunction|ClearLevel false)
        (Default|ShowLevelCompleteScreen (Variables|Default|GetMessagesDisplay))
        (bind _outactors (Actor|GetAllActorsOfClass "/Game/FlickerGame/Blueprints/CommandBase.CommandBase_C"))
        (Default|HideBar _outactors)
        (Utilities|FlowControl|Delay 3.0)
        (Utilities|FlowControl|Sequence
          (:then_0
            (bind _outactors_2 (Actor|GetAllActorsOfClass "/Game/FlickerGame/Blueprints/CommandBase.CommandBase_C"))
            (Actor|DestroyActor _outactors_2))
          (:then_1
            (Default|Shrink (Variables|Default|GetTerrain))
            (Utilities|FlowControl|Delay 2.0)
            (CallFunction|LoadNextLevel)))
        (else
          ;[1 1 1] Check defeat
          (if (Utilities|IsValid _playerbase)
            (if (Variables|/Game/FlickerGame/Blueprints/CommandBase.CommandBase_C|GetIsDead _playerbase)
              ;[1 1 1] shows defeat screen and goes to game over state
              (Variables|Default|SetState "NewEnumerator0")
              (CallFunction|ClearLevel false)
              (bind _outactors_3 (Actor|GetAllActorsOfClass "/Game/FlickerGame/Blueprints/CommandBase.CommandBase_C"))
              (Default|HideBar _outactors_3)
              (Audio|Components|Audio|Stop (Variables|Default|GetBackgroundMusic))
              (Utilities|FlowControl|Delay 3.0)
              (Utilities|FlowControl|Sequence
                (:then_0
                  (bind _outactors_4 (Actor|GetAllActorsOfClass "/Game/FlickerGame/Blueprints/CommandBase.CommandBase_C"))
                  (Actor|DestroyActor _outactors_4))
                (:then_1
                  (Default|ShowLevelFailedScreen (Variables|Default|GetMessagesDisplay))
                  (Default|Shrink (Variables|Default|GetTerrain))
                  (Utilities|FlowControl|Delay 4.0)
                  (Default|ShowGameOverScreen (Variables|Default|GetMessagesDisplay))
                  (Utilities|FlowControl|Delay 5.0)
                  (if (Utilities|Enum|Equal(Enum) (Variables|Default|GetState) "NewEnumerator0")
                    (Default|HideGameOverMessage (Variables|Default|GetMessagesDisplay))
                    (Default|ShowScreen (Variables|Default|GetGameTitleScreen)))))
              (else
                ;[0.27 0.27 0.27] Spawn level units
                (while (and (< (Variables|Default|GetLevelUnitIndex) (Utilities|Array|Length (Variables|Default|GetCurrentLevelData))) (> (Actor|GetGameTimeSinceCreation) (+ _spawntime (+ (Variables|Default|GetLevelStartTime) 4.0))))
                  (if (Utilities|Enum|Equal(Enum) _team "NewEnumerator0")
                    (Default|SpawnUnit (Variables|Default|GetPlayerSpawnRegion) _type)
                    (else
                      (Default|SpawnUnit (Variables|Default|GetEnemySpawnRegion) _type)))
                  (Math|Integer|IncrementInt (Variables|Default|GetLevelUnitIndex)))))))))))

(fn ConstructionScript)

(fn LoadLevel
  (params (LevelIndex :type Integer))
  (bind _currentleveldata (Variables|Default|GetCurrentLevelData))
  (bind _currentleveldata_2 (Variables|Default|GetCurrentLevelData))
  (bind _backgroundmusic (Variables|Default|GetBackgroundMusic))
  (bind _currentleveldata_3 (Variables|Default|GetCurrentLevelData))
  (bind _output_get (Variables|Default|SetcurrentLevel LevelIndex))
  (Utilities|FlowControl|Sequence
    (:then_0
      (CallFunction|ClearLevel false)
      (Default|HideGameOverScreen (Variables|Default|GetMessagesDisplay)))
    (:then_1
      ;[1 1 1] spawns bases
      (bind _returnvalue (Game|SpawnActorfromClass "/Game/FlickerGame/Blueprints/CommandBase.CommandBase_C" (Math|Conversions|ToTransform(Vector) (Variables|Default|GetPlayerBaseLocation)) "AdjustIfPossibleButAlwaysSpawn" 0 0))
      (Default|SetTeam _returnvalue "NewEnumerator0")
      (Variables|Default|SetPlayerBase _returnvalue))
    (:then_2
      (bind _returnvalue_2 (Game|SpawnActorfromClass "/Game/FlickerGame/Blueprints/CommandBase.CommandBase_C" (Math|Conversions|ToTransform(Vector) (Variables|Default|GetEnemyBaseLocation)) "AdjustIfPossibleButAlwaysSpawn" 0 0))
      (Default|SetTeam _returnvalue_2 "NewEnumerator1")
      (Variables|Default|SetEnemyBase _returnvalue_2))
    (:then_3
      (Default|Grow (Variables|Default|GetTerrain))
      (Variables|Default|SetLevelStartTime (Actor|GetGameTimeSinceCreation))
      (Variables|Default|SetState "NewEnumerator1")
      (Variables|Default|SetLevelUnitIndex 0)
      (Default|ShowLevelStartScreen (Variables|Default|GetMessagesDisplay) (Variables|Default|GetcurrentLevel))
      (if (not (Audio|Components|Audio|IsPlaying _backgroundmusic))
        (Audio|Components|Audio|Play _backgroundmusic 0.0)
        (Audio|Components|Audio|FadeIn _backgroundmusic 2.0 0.6 0.0 :!class /Script/Engine.AudioComponent)))
    (:then_4
      (switch int _output_get
        (:Default
          ;[1 1 1] Level 0
          (Utilities|Array|Clear _currentleveldata :!label _label)
          (Utilities|Array|Add _currentleveldata (Utilities|Struct|MakeUnitData "/Game/FlickerGame/Blueprints/SoldierUnit.SoldierUnit_C" "NewEnumerator0" 0.0))
          (Utilities|Array|Add _currentleveldata (Utilities|Struct|MakeUnitData "/Game/FlickerGame/Blueprints/SoldierUnit.SoldierUnit_C" "NewEnumerator1" 2.0))
          (Utilities|Array|Add _currentleveldata (Utilities|Struct|MakeUnitData "/Game/FlickerGame/Blueprints/SoldierUnit.SoldierUnit_C" "NewEnumerator0" 4.0)))
        (:0
          (goto _label))
        (:1
          ;[1 1 1] Level 1
          (Utilities|Array|Clear _currentleveldata_2)
          (Utilities|Array|Add _currentleveldata_2 (Utilities|Struct|MakeUnitData "/Game/FlickerGame/Blueprints/SoldierUnit.SoldierUnit_C" "NewEnumerator0" 0.0))
          (Utilities|Array|Add _currentleveldata_2 (Utilities|Struct|MakeUnitData "/Game/FlickerGame/Blueprints/SoldierUnit.SoldierUnit_C" "NewEnumerator1" 0.0))
          (Utilities|Array|Add _currentleveldata_2 (Utilities|Struct|MakeUnitData "/Game/FlickerGame/Blueprints/RocketSoldierUnit.RocketSoldierUnit_C" "NewEnumerator0" 2.0))
          (Utilities|Array|Add _currentleveldata_2 (Utilities|Struct|MakeUnitData "/Game/FlickerGame/Blueprints/RocketSoldierUnit.RocketSoldierUnit_C" "NewEnumerator0" 2.0)))
        (:2
          ;[1 1 1] level 2
          (Utilities|Array|Clear _currentleveldata_3)
          (Utilities|Array|Add _currentleveldata_3 (Utilities|Struct|MakeUnitData "/Game/FlickerGame/Blueprints/SoldierUnit.SoldierUnit_C" "NewEnumerator1" 0.0))
          (Utilities|Array|Add _currentleveldata_3 (Utilities|Struct|MakeUnitData "/Game/FlickerGame/Blueprints/SoldierUnit.SoldierUnit_C" "NewEnumerator1" 2.0))
          (Utilities|Array|Add _currentleveldata_3 (Utilities|Struct|MakeUnitData "/Game/FlickerGame/Blueprints/SoldierUnit.SoldierUnit_C" "NewEnumerator0" 4.0))
          (Utilities|Array|Add _currentleveldata_3 (Utilities|Struct|MakeUnitData "/Game/FlickerGame/Blueprints/SoldierUnit.SoldierUnit_C" "NewEnumerator1" 6.0))
          (Utilities|Array|Add _currentleveldata_3 (Utilities|Struct|MakeUnitData "/Game/FlickerGame/Blueprints/SoldierUnit.SoldierUnit_C" "NewEnumerator1" 6.0)))))))

(fn ClearLevel
  (params (destory%20bases :type Boolean))
  (Utilities|FlowControl|Sequence
    (:then_0
      ;[1 1 1] destroy prjectiles
      (bind _outactors (Actor|GetAllActorsOfClass "/Game/FlickerGame/Blueprints/Projectile.Projectile_C"))
      (for _array_element _outactors
        (Actor|DestroyActor _array_element)))
    (:then_1
      ;[1 1 1] destroy units
      (bind _outactors_2 (Actor|GetAllActorsOfClass "/Game/FlickerGame/Blueprints/BaseUnitBP.BaseUnitBP_C"))
      (for _array_element_2 _outactors_2
        (if (Utilities|IsValid (Variables|/Game/FlickerGame/Blueprints/BaseUnitBP.BaseUnitBP_C|GetWeapon _array_element_2))
          (Actor|DestroyActor (Variables|/Game/FlickerGame/Blueprints/BaseUnitBP.BaseUnitBP_C|GetWeapon _array_element_2)))
        (Actor|DestroyActor _array_element_2)))
    (:then_2
      (if destory%20bases
        ;[1 1 1] destroy bases
        (bind _outactors_3 (Actor|GetAllActorsOfClass "/Game/FlickerGame/Blueprints/CommandBase.CommandBase_C"))
        (Actor|DestroyActor _outactors_3)))))

(fn ResetCurrentLevel
  (CallFunction|ClearLevel false)
  (CallFunction|LoadLevel (Variables|Default|GetcurrentLevel)))

(fn LoadNextLevel
  (Math|Integer|IncrementInt (Variables|Default|GetcurrentLevel)
    (:%20%20
      (if (>= (Variables|Default|GetcurrentLevel) (Variables|Default|GetLevelsCount))
        (Variables|Default|SetcurrentLevel 0))
      (CallFunction|ClearLevel true)
      (CallFunction|LoadLevel (Variables|Default|GetcurrentLevel)))))

(fn StartNewGame
  (bind _output_get (Variables|Default|SetcurrentLevel 0))
  (CallFunction|LoadLevel _output_get)
  (Default|HideScreen (Variables|Default|GetGameTitleScreen)))