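; CommandBase is a destructible base actor in FlickerGame with health and a configurable color.
; AffectHealth subtracts the given delta from Health and sets IsDead once it reaches zero or below.
; Tick polls that flag and destroys the actor.
; The construction script applies the Color variable through a dynamic material instance on the CommandBase component.
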(event EventAffectHealth
  (params (delta :type Float%20%28single-precision%29))
  (bind _output_get (Variables|Default|SetHealth (- (Variables|Default|GetHealth) delta)))
  (if (<= _output_get 0.0)
    (Variables|Default|SetIsDead true)))

(event EventTick
  (params (DeltaSeconds :type Float%20%28single-precision%29))
  (if (Variables|Default|GetIsDead)
    (Actor|DestroyActor)))

(fn ConstructionScript
  (bind _commandbase (Variables|Default|GetCommandBase))
  (bind _returnvalue (Rendering|Material|CreateDynamicMaterialInstance _commandbase 0 0 :!class /Script/Engine.PrimitiveComponent))
  (Rendering|Material|SetVectorParameterValue _returnvalue "Color" (Variables|Default|GetColor) :!class /Script/Engine.MaterialInstanceDynamic)
  (Rendering|Material|SetMaterial _commandbase 0 _returnvalue))