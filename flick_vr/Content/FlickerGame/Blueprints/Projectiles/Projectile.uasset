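; Laser projectile Blueprint that damages IDamagable actors on overlap, sparing units on its own team.
; BaseUnitBP targets are hit only if their Team differs, while any other damagable actor is always hit through the AffectHealthMessage interface call.
; A hit spawns an explosion, removes the mesh and collision, and plays a hit sound with pitch randomized at BeginPlay, then destroys the actor after a short delay.
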(event Collision|EventActorBeginOverlap
  (params (OtherActor :type Actor%20Object%20Reference))
  (if (Utilities|DoesObjectImplementInterface OtherActor "/Script/flick_vr.IDamagable")
    (bind _asbase_unit_bp (Utilities|Casting|CastToBaseUnitBP OtherActor)
      (:then
        (if (Utilities|Enum|NotEqual(Enum) (Variables|/Game/FlickerGame/Blueprints/Units/BaseUnitBP.BaseUnitBP_C|GetTeam _asbase_unit_bp) (Variables|Default|GetTeam))
          (Class|IDamagable|AffectHealth(Message) OtherActor (Variables|Default|GetDamage) :!label _label)
          (Effects|SpawnEmitteratLocation "/Game/FlickerGame/Particles/P_HalfMoonExplosion.P_HalfMoonExplosion" (Transformation|GetWorldLocation (Variables|Default|GetDefaultSceneRoot)))
          (Components|DestroyComponent (Variables|Default|GetLaserMesh))
          (Audio|Components|Audio|Play (Variables|Default|Gethitsound) 0.0)
          (Utilities|FlowControl|Delay 1.0)
          (Actor|DestroyActor)))
      (:CastFailed
        (goto _label)))))

(event EventBeginPlay
  (Audio|Components|Audio|SetPitchMultiplier (Variables|Default|Gethitsound) (Math|Random|RandomFloatinRange 0.8 1.5)))

(fn ConstructionScript)