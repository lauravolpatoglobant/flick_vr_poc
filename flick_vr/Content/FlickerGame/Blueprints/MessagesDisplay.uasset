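; MessagesDisplay shows holographic 3D-mesh messages for game over, push start, level intro with get ready, and mission accomplished or failed.
; BeginPlay hides level screens, starts push-start blinking and drives hologram intensity through timelines on dynamic M_Hologram instances, one shared by several meshes.
; Show events play sounds and timelines that move and scale each message, then hide it on finish.
; Level intro selects a mesh by LevelId and blinks get ready.
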(event Custom|ShowLevelStartScreen
  (params (LevelId :type Integer))
  (bind _pushstart (Variables|Default|Getpushstart))
  (bind _getreadymesh (Variables|Default|Getgetreadymesh))
  (bind _levelmesh (Variables|Default|GetLevelMesh))
  ;[1 1 1] shows level start screen
  (Utilities|FlowControl|Sequence
    (:then_0
      (Timeline|Timeline_4 Stop
        (:Show%20push%20start
          (Rendering|SetVisibility _pushstart true true))
        (:Hide%20push%20start
          (Rendering|SetVisibility _pushstart false true))))
    (:then_1
      (Rendering|SetVisibility (Variables|Default|GetPushStartPivot) false true))
    (:then_2
      (Audio|Components|Audio|Play (Variables|Default|GetLevelStartSound) 0.0)
      (switch int LevelId
        (:Default
          (Components|StaticMesh|SetStaticMesh _levelmesh "/Game/FlickerGame/Meshes/level01.level01" :!label _label))
        (:0
          (goto _label))
        (:1
          (Components|StaticMesh|SetStaticMesh _levelmesh "/Game/FlickerGame/Meshes/level02.level02"))
        (:2
          (Components|StaticMesh|SetStaticMesh _levelmesh "/Game/FlickerGame/Meshes/level03.level03"))
        (:3
          (Components|StaticMesh|SetStaticMesh _levelmesh "/Game/FlickerGame/Meshes/level04.level04")))
      (Utilities|FlowControl|Delay 0.5)
      (Utilities|FlowControl|Sequence
        (:then_0
          (bind (_direction _position _get_ready_position) (Timeline|LevelTimeline Stop)
            (:Update
              (Transformation|SetRelativeLocation (Variables|Default|GetLevel) (Math|Vector|MakeVector 0.0 0.0 (+ (* _position 2e+01) -2e+01)) false false)
              (Transformation|SetRelativeScale3D (Variables|Default|GetLevelMesh) (Math|Conversions|ToVector(Float) _position))
              (Transformation|SetRelativeLocation (Variables|Default|Getgetreadypivot) (Math|Vector|MakeVector 0.0 15.0 (+ (* _get_ready_position 2e+01) -2e+01)) false false)
              (Transformation|SetRelativeScale3D (Variables|Default|Getgetreadymesh) (Math|Conversions|ToVector(Float) (* _get_ready_position 0.5))))
            (:Finished
              (CallFunction|HideLevelStartScreen))
            (:Start%20blinking%20
              (Timeline|Timeline_5 PlayFromStart
                (:Show%20push%20start
                  (Rendering|SetVisibility _getreadymesh true true :!label _label_2))
                (:Hide%20push%20start
                  (Rendering|SetVisibility _getreadymesh false true))))
            (:Stop%20Blinking
              (Utilities|FlowControl|Sequence
                (:then_0
                  (Timeline|Timeline_5 Stop))
                (:then_1
                  (goto _label_2))))))
        (:then_1
          (Rendering|SetVisibility (Variables|Default|GetLevel) true true)
          (Utilities|FlowControl|Sequence
            (:then_0
              (Timeline|LevelTimeline PlayFromStart))
            (:then_1
              (Audio|Components|Audio|Play (Variables|Default|GetMessage) 0.0)
              (Utilities|FlowControl|Delay 0.6)
              (Audio|Components|Audio|Play (Variables|Default|GetMessage) 0.0)
              (Audio|Components|Audio|Play (Variables|Default|Getgetready) 0.0)
              (Utilities|FlowControl|Delay 1.6)
              (Audio|Components|Audio|Play (Variables|Default|GetMessage) 0.0)
              (Utilities|FlowControl|Delay 0.15)
              (Audio|Components|Audio|Play (Variables|Default|GetMessage) 0.0))))))))

(event Custom|ShowLevelCompleteScreen
  ;[1 1 1] showls level complete screen
  (Utilities|FlowControl|Delay 0.5)
  (Audio|Components|Audio|Play (Variables|Default|Getlevelfinishsound) 0.0)
  (Utilities|FlowControl|Sequence
    (:then_0
      (bind _position (Timeline|Timeline_2 Stop)
        (:Update
          (Transformation|SetRelativeLocation (Variables|Default|Getlevelcomplete) (Math|Vector|MakeVector 0.0 0.0 (+ (* _position 2e+01) -2e+01)) false false)
          (Transformation|SetRelativeScale3D (Variables|Default|Getmissionaccomplished) (Math|Conversions|ToVector(Float) _position)))
        (:Finished
          (CallFunction|HideLevelCompleteScreen))))
    (:then_1
      (Rendering|SetVisibility (Variables|Default|Getlevelcomplete) true true)
      (Timeline|Timeline_2 PlayFromStart))))

(event Custom|ShowLevelFailedScreen
  ;[1 1 1] showls level failed screen
  (Utilities|FlowControl|Delay 0.5)
  (Audio|Components|Audio|Play (Variables|Default|Getlevelfinishsound) 0.0)
  (Utilities|FlowControl|Sequence
    (:then_0
      (bind _position (Timeline|Timeline_3 Stop)
        (:Update
          (Transformation|SetRelativeLocation (Variables|Default|Getmissionfailedpivot) (Math|Vector|MakeVector 0.0 0.0 (+ (* _position 2e+01) -2e+01)) false false)
          (Transformation|SetRelativeScale3D (Variables|Default|Getmissionfailed) (Math|Conversions|ToVector(Float) _position)))
        (:Finished
          (CallFunction|HideLevelFailedScreen))))
    (:then_1
      (Rendering|SetVisibility (Variables|Default|Getmissionfailedpivot) true true)
      (Timeline|Timeline_3 PlayFromStart))))

(event EventBeginPlay
  (bind _pushstart (Variables|Default|Getpushstart))
  (Utilities|FlowControl|Sequence
    (:then_0
      ;[1 1 1] sets game over animation
      (bind _returnvalue (Rendering|Material|CreateDynamicMaterialInstance "/Game/FlickerGame/Materials/M_Hologram.M_Hologram" :!class /Script/Engine.KismetMaterialLibrary))
      (Rendering|Material|SetMaterial (Variables|Default|GetGameOverMesh) 0 _returnvalue)
      (bind _output (Timeline|Timeline_0 Play)
        (:Update
          (Transformation|SetRelativeLocation (Variables|Default|GetGameOverPivot) (Math|Vector|MakeVector 0.0 0.0 (* _output 1e+01)) false false)
          (Rendering|Material|SetScalarParameterValue _returnvalue "Intensity" _output :!class /Script/Engine.MaterialInstanceDynamic))))
    (:then_1
      (Timeline|Timeline_4 Play
        (:Show%20push%20start
          (Rendering|SetVisibility _pushstart true true))
        (:Hide%20push%20start
          (Rendering|SetVisibility _pushstart false true))))
    (:then_2
      ;[1 1 1] sets dynamic materials animations
      (bind _returnvalue_2 (Rendering|Material|CreateDynamicMaterialInstance "/Game/FlickerGame/Materials/M_Hologram.M_Hologram" :!class /Script/Engine.KismetMaterialLibrary))
      (Rendering|Material|SetMaterial (Variables|Default|Getpushstart) 1 _returnvalue_2)
      (bind _output_2 (Timeline|Timeline_1 Play)
        (:Update
          (Rendering|Material|SetScalarParameterValue _returnvalue_2 "Intensity" _output_2 :!class /Script/Engine.MaterialInstanceDynamic))))
    (:then_3
      (CallFunction|HideLevelStartScreen)
      (CallFunction|HideLevelCompleteScreen)
      (CallFunction|HideLevelFailedScreen)
      (CallFunction|ShowGameOverScreen)
      (CallFunction|HideGameOverMessage))))

(fn ConstructionScript)

(fn HideGameOverScreen
  (Rendering|SetVisibility (Variables|Default|GetGameOverMesh) false true)
  (Audio|Components|Audio|Stop (Variables|Default|Getgameoverhum)))

(fn ShowGameOverScreen
  (Rendering|SetVisibility (Variables|Default|GetGameOverMesh) true false)
  (Audio|Components|Audio|Play (Variables|Default|Getgameoverhum) 0.0))

(fn HideLevelStartScreen
  (Rendering|SetVisibility (Variables|Default|GetLevel) false true))

(fn HideLevelCompleteScreen
  (Rendering|SetVisibility (Variables|Default|Getlevelcomplete) false true))

(fn HideLevelFailedScreen
  (Rendering|SetVisibility (Variables|Default|Getmissionfailedpivot) false true))

(fn HideGameOverMessage
  (Rendering|SetVisibility (Variables|Default|GetGameOverPivot) false true))