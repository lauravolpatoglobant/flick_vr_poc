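; Rocket launcher weapon for FlickerGame, built on a parent Blueprint that it calls for begin play, tick and construction.
; On begin play it assigns the MenuExit_Stereo sound to its shoot sound component and lowers the volume.
; Its SpawnProjectile event spawns a RocketProjectile2 at the projectile spawn point's world transform and passes the weapon's team to it.
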(event EventTick
  (params (DeltaSeconds :type Float%20%28single-precision%29))
  (|CallParentFunction DeltaSeconds))

(event EventBeginPlay
  (bind _shootsound (Variables|Default|Getshootsound))
  (|CallParentFunction)
  (Audio|Components|Audio|SetSound _shootsound "/Game/FlickerGame/Audio/MenuExit_Stereo.MenuExit_Stereo")
  (Audio|Components|Audio|SetVolumeMultiplier _shootsound 0.3 :!class /Script/Engine.AudioComponent))

(event EventSpawnProjectile
  (Game|SpawnActorfromClass "/Game/FlickerGame/Blueprints/Projectiles/RocketProjectile2.RocketProjectile2_C" (Transformation|GetWorldTransform (Variables|Default|GetProjectileSpawnPoint)) "Undefined" 0 (Variables|Default|GetTeam) 0))

(fn ConstructionScript
  (|CallParentFunction))