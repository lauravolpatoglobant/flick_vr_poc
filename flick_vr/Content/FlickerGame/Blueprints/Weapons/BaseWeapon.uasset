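; Base weapon Blueprint that handles hold-to-fire automatic shooting.
; StartFiring and StopFiring toggle a firing flag, which Tick checks against a game-time cooldown to call SpawnProjectile and play the shoot sound.
; SpawnProjectile only prints a debug string here, so no projectile is created.
; The shoot sound's pitch is randomized once at BeginPlay, not on every shot.
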(event Custom|StopFiring
  (Variables|Default|SetIsFiring false))

(event Custom|StartFiring
  (Variables|Default|SetIsFiring true))

(event EventTick
  (params (DeltaSeconds :type Float%20%28single-precision%29))
  (if (Variables|Default|GetIsFiring)
    (Math|Float|CompareFloat (Variables|Default|GetCooldownTimer) (Utilities|Time|GetGameTimeinSeconds)
      (:<
        (CallFunction|SpawnProjectile)
        (Variables|Default|SetCooldownTimer (+ (Utilities|Time|GetGameTimeinSeconds) (Variables|Default|GetFireCooldown)))
        (Audio|Components|Audio|Play (Variables|Default|Getshootsound) 0.0)))))

(event EventBeginPlay
  (Audio|Components|Audio|SetPitchMultiplier (Variables|Default|Getshootsound) (Math|Random|RandomFloatinRange 0.8 1.5)))

(fn ConstructionScript)

(fn SpawnProjectile
  (Development|PrintString "SpawningProjectile"))