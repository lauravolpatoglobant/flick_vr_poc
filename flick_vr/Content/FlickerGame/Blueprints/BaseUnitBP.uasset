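; Base combat unit that marches on the opposing team's command base and fights enemy units it meets on the way.
; Each tick it keeps a living enemy or sphere-traces for one, defaulting to the base, then fires within range or moves straight toward it without pathfinding.
; SetTeam tints the body through a dynamic material and finds the base.
; At zero health it ignores pawns, detaches its controller, blinks via timeline, and is destroyed.
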(event EventAffectHealth
  (params (delta :type Float%20%28single-precision%29))
  (bind _capsulecomponent (Variables|Default|GetCapsuleComponent))
  (bind _weapon (Variables|Default|GetWeapon))
  (bind _defaultsceneroot (Variables|/Game/FlickerGame/Blueprints/Weapon.Weapon_C|GetDefaultSceneRoot _weapon))
  ;[1 1 1] Reduce health on hit and destroy the actor when health reaches 0
  (bind _output_get (Variables|Default|SetHealth (- (Variables|Default|GetHealth) delta)))
  (if (<= _output_get 0.0)
    (Variables|Default|SetIsDead true)
    (Collision|SetCollisionResponsetoChannel _capsulecomponent "ECC_WorldDynamic" "ECR_Ignore")
    (Collision|SetCollisionResponsetoChannel _capsulecomponent "ECC_Pawn" "ECR_Ignore")
    (Class|Pawn|DetachfromControllerPendingDestroy)
    (Utilities|FlowControl|Delay 1.5)
    (Utilities|FlowControl|Sequence
      (:then_0
        (Utilities|FlowControl|Delay 2.0)
        (Utilities|FlowControl|Sequence
          (:then_0
            ;[1 1 1] makes unit to blink
            (Timeline|Timeline_0 Stop
              (:show
                (Rendering|SetVisibility _defaultsceneroot true true))
              (:hide
                (Rendering|SetVisibility _defaultsceneroot false true))))
          (:then_1
            (Actor|DestroyActor (Variables|Default|GetWeapon))
            (Actor|DestroyActor))))
      (:then_1
        (Timeline|Timeline_0 Play)))))

(event EventBeginPlay
  ;[1 1 1] Find base to attack
  (if (Utilities|Enum|NotEqual(Enum) (Variables|Default|GetTeam) "NewEnumerator2")
    (CallFunction|FindEnemyBase)))

(event EventTick
  (params (DeltaSeconds :type Float%20%28single-precision%29))
  (bind _targettoattack (Variables|Default|GetTargetToAttack))
  (Utilities|IsUnitAlive
    (:True
      (CallFunction|SetTargettoAttack)
      (Utilities|HasValidTarget _targettoattack
        (:Valid
          (Utilities|IsTargetinFireRange _targettoattack
            (:In%20range
              (CallFunction|AttackTarget _targettoattack))
            (:NotInRange
              (CallFunction|MovetoTarget DeltaSeconds _targettoattack)
              (Default|StopFiring (Variables|Default|GetWeapon) :!label _label))))
        (:NotValid
          (goto _label))))
    (:False
      (goto _label))))

(fn ConstructionScript)

(fn SetTeam
  (params (NewTeam :type Teams%20Enum) (Target :type Actor%20Object%20Reference))
  (Variables|Default|SetTeam NewTeam)
  (CallFunction|SetColor)
  (bind _basefound (CallFunction|FindEnemyBase))
  (Variables|Default|SetHasTarget _basefound))

(fn FindEnemyBase
  (if (Utilities|Enum|NotEqual(Enum) (Variables|Default|GetTeam) "NewEnumerator2")
    (bind _outactors (Actor|GetAllActorsOfClass "/Game/FlickerGame/Blueprints/CommandBase.CommandBase_C"))
    (bind _array_element (Utilities|Array|ForEachLoopwithBreak _outactors)
      (:LoopBody
        (if (Utilities|Enum|NotEqual(Enum) (Variables|/Game/FlickerGame/Blueprints/CommandBase.CommandBase_C|GetTeam _array_element) (Variables|Default|GetTeam))
          (Variables|Default|SetBaseToAttack _array_element)
          (bind _output_get (Variables|Default|SetHasTarget true))
          (return _output_get)))
      (:Completed
        (return false)))
    (else
      (return false))))

(fn FaceTarget
  (params (Target :type Actor%20Object%20Reference))
  (Utilities|HasValidTarget Target
    (:Valid
      (Transformation|SetWorldRotation (Variables|Character|GetMesh) (Math|Rotator|MakeRotator 0.0 0.0 (+ (.Yaw (Math|Rotator|BreakRotator (Math|Rotator|FindLookatRotation (Transformation|GetActorLocation) (Transformation|GetActorLocation Target)))) -9e+01)) false false))))

(fn AttackTarget
  (params (Target :type Actor%20Object%20Reference))
  (CallFunction|FaceTarget Target)
  (Default|StartFiring (Variables|Default|GetWeapon)))

(fn MovetoTarget
  (params (TimeDelta :type Float%20%28single-precision%29) (Target :type Actor%20Object%20Reference))
  (bind _returnvalue (Transformation|GetActorLocation))
  (Transformation|SetActorLocation (+ (* (* (Math|Vector|Normalize (- (Transformation|GetActorLocation Target) _returnvalue)) TimeDelta) (Variables|Default|GetSpeed)) _returnvalue) false false)
  (CallFunction|FaceTarget Target))

(fn FindNextEnemy
  (bind _returnvalue (Transformation|GetActorLocation))
  (bind _outhits (Collision|MultiSphereTraceForObjects _returnvalue _returnvalue 1e+02 (Variables|Default|GetTriggerObjectTypes) false 0 "None"))
  (bind _array_element (Utilities|Array|ForEachLoopwithBreak _outhits :!label _label)
    (:LoopBody
      (bind _asbase_unit_bp (Utilities|Casting|CastToBaseUnitBP (.HitActor (Collision|BreakHitResult _array_element))))
      (bind _result (CallFunction|IsUnitTeamDefined _asbase_unit_bp))
      (if _result
        (Utilities|IsValid _asbase_unit_bp
          (:Is%20Valid
            (if (Utilities|Enum|NotEqual(Enum) (Variables|BaseUnitBP_C|GetTeam _asbase_unit_bp) (Variables|Default|GetTeam))
              (Variables|Default|SetEnemyToFight _asbase_unit_bp)
              (Variables|Default|SetIsFighting true)
              (goto _label Break))))))))

(fn IsUnitTeamDefined
  (params (Unit :type Base%20Unit%20BP%20Object%20Reference))
  (return (Utilities|Enum|NotEqual(Enum) (Variables|BaseUnitBP_C|GetTeam Unit) "NewEnumerator2")))

(fn IsEnemyStillAlive
  (params (Enemy :type Actor%20Object%20Reference))
  (bind _asbase_unit_bp (Utilities|Casting|CastToBaseUnitBP Enemy)
    (:then
      (Utilities|IsValid _asbase_unit_bp
        (:Is%20Valid
          (if (Variables|/Script/flick_vr.BaseUnit|GetIsDead _asbase_unit_bp)
            _
            (else
              (return true))))
        (:Is%20Not%20Valid
          _)))
    (:CastFailed
      _))
  (return false))

(fn SetTargettoAttack
  (bind _result (CallFunction|IsEnemyStillAlive (Variables|Default|GetEnemyToFight)))
  (if _result
    (Variables|Default|SetTargetToAttack (Variables|Default|GetEnemyToFight))
    (else
      (Variables|Default|SetIsFighting false)
      (CallFunction|FindNextEnemy)
      (Variables|Default|SetTargetToAttack (Variables|Default|GetBaseToAttack)))))

(fn SetColor
  (switch Utilities|FlowControl|Switch|SwitchonTeams (Variables|Default|GetTeam)
    (:NewEnumerator0
      (Variables|Default|SetUnitColor "(R=0.000000,G=0.000000,B=0.800000,A=1.000000)"))
    (:NewEnumerator1
      (Variables|Default|SetUnitColor "(R=0.800000,G=0.000000,B=0.000000,A=1.000000)")))
  (bind _returnvalue (Rendering|Material|CreateDynamicMaterialInstance (Variables|Character|GetMesh) 0 0 :!class /Script/Engine.PrimitiveComponent))
  (Rendering|Material|SetVectorParameterValue _returnvalue "BodyColor" (Variables|Default|GetUnitColor) :!class /Script/Engine.MaterialInstanceDynamic))