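; SpawnEffect is a self-destructing visual effect actor that shows an animated spawn ring with a light.
; On BeginPlay it sets its root to a fixed world height and applies a dynamic SpawnRing material to its static mesh.
; A timeline then drives the flattened mesh's horizontal scale, the material's Alpha parameter, and the light's intensity and attenuation radius.
; The actor destroys itself when the timeline finishes.
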(event EventBeginPlay
  (bind _light (Variables|Default|GetLight))
  (bind _defaultsceneroot (Variables|Default|GetDefaultSceneRoot))
  (bind _returnvalue (Transformation|GetWorldLocation _defaultsceneroot))
  (bind (_x _y) (Math|Vector|BreakVector _returnvalue))
  (Transformation|SetWorldLocation _defaultsceneroot (Math|Vector|MakeVector _x _y 1e+02) false false)
  (bind _returnvalue_2 (Rendering|Material|CreateDynamicMaterialInstance "/Game/FlickerGame/Materials/SpawnRing.SpawnRing" :!class /Script/Engine.KismetMaterialLibrary))
  (Rendering|Material|SetMaterial (Variables|Default|GetStaticMesh) 0 _returnvalue_2)
  (bind (_direction _scale _alpha _light_intesnsity) (Timeline|Timeline_0 Play)
    (:Update
      (Transformation|SetWorldScale3D (Variables|Default|GetStaticMesh) (Math|Vector|MakeVector (* _scale 1.0) (* _scale 1.0) 0.0))
      (Rendering|Material|SetScalarParameterValue _returnvalue_2 "Alpha" _alpha :!class /Script/Engine.MaterialInstanceDynamic)
      (Rendering|Components|Light|SetIntensity _light (* _light_intesnsity 2e+02))
      (Rendering|Lighting|SetAttenuationRadius _light (* _light_intesnsity 2e+01)))
    (:Finished
      (Actor|DestroyActor))))

(fn ConstructionScript)