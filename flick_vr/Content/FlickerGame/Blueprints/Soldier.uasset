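; Soldier unit that marches toward a CommandBase and stops once within fire distance.
; On BeginPlay it picks the base whose actor tag matches BaseTagToSearch.
; Each Tick it moves straight at the base without sweep and yaws its mesh to face it.
; The range check compares only world X in the positive direction, setting ReachedTarget and halting movement; no firing logic is present.
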(event EventBeginPlay
  ;[1 1 1] Find a reference to the base we should attack
  (bind _outactors (Actor|GetAllActorsOfClass "/Game/FlickerGame/Blueprints/CommandBase.CommandBase_C"))
  (for _array_element _outactors
    (if (Actor|ActorHasTag _array_element (Utilities|String|StringToName (Variables|Default|GetBaseTagToSearch)))
      (Variables|Default|SetBaseToAttack _array_element))))

(event EventTick
  (params (DeltaSeconds :type Float%20%28single-precision%29))
  (bind _returnvalue (Transformation|GetActorLocation))
  (bind _basetoattack (Variables|Default|GetBaseToAttack))
  (bind _returnvalue_2 (Transformation|GetActorLocation _basetoattack))
  ;[1 1 1] Check if we are on fire distance from the base
  (if (>= (+ (.x (Transformation|GetActorLocation)) (Variables|Default|GetFireDistance)) (.x (Transformation|GetActorLocation (Variables|Default|GetBaseToAttack))))
    (Variables|Default|SetReachedTarget true)
    (else
      (Variables|Default|SetReachedTarget false)
      (Transformation|SetActorLocation (+ (* (* (Math|Vector|Normalize (- _returnvalue_2 _returnvalue)) DeltaSeconds) (Variables|Default|GetSpeed)) _returnvalue) false false)
      (Transformation|SetWorldRotation (Variables|Character|GetMesh) (Math|Rotator|MakeRotator 0.0 0.0 (+ (.Yaw (Math|Rotator|BreakRotator (Math|Rotator|FindLookatRotation _returnvalue _returnvalue_2))) -9e+01)) false false))))

(fn ConstructionScript)