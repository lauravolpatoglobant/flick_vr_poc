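; Terrain actor for FlickerGame whose surface can be grown or shrunk through a material effect.
; BeginPlay puts a dynamic M_DefaultTerrain instance on the terrain mesh and starts its Aperture parameter at zero.
; Grow plays audio and runs a timeline from the start, feeding its doubled output into Aperture.
; Shrink plays the same audio and reverses that timeline to close the effect.
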(event Custom|Grow
  (Audio|Components|Audio|Play (Variables|Default|GetAudio) 0.0)
  (Utilities|FlowControl|Sequence
    (:then_0
      (bind _output (Timeline|Timeline_0 Stop)
        (:Update
          (Rendering|Material|SetScalarParameterValue (Variables|Default|GetTerrainMaterial) "Aperture" (* _output 2.0) :!class /Script/Engine.MaterialInstanceDynamic))))
    (:then_1
      (Timeline|Timeline_0 PlayFromStart))))

(event Custom|Shrink
  (Audio|Components|Audio|Play (Variables|Default|GetAudio) 0.0)
  (Utilities|FlowControl|Sequence
    (:then_0
      (bind _output (Timeline|Timeline_0 Stop)
        (:Update
          (Rendering|Material|SetScalarParameterValue (Variables|Default|GetTerrainMaterial) "Aperture" (* _output 2.0) :!class /Script/Engine.MaterialInstanceDynamic))))
    (:then_1
      (Timeline|Timeline_0 Reverse))))

(event EventBeginPlay
  (bind _returnvalue (Rendering|Material|CreateDynamicMaterialInstance "/Game/FlickerGame/Materials/M_DefaultTerrain.M_DefaultTerrain" :!class /Script/Engine.KismetMaterialLibrary))
  (Variables|Default|SetTerrainMaterial _returnvalue)
  (Rendering|Material|SetMaterial (Variables|Default|GetTerrainMesh) 0 _returnvalue)
  (Rendering|Material|SetScalarParameterValue _returnvalue "Aperture" 0.0 :!class /Script/Engine.MaterialInstanceDynamic))

(fn ConstructionScript)