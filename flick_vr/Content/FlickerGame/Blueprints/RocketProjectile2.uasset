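; RocketProjectile2 is a rocket projectile Blueprint that damages non-friendly damagable actors on overlap.
; On overlap it checks the IDamagable interface and Friendly tag, then sends Damage through AffectHealthMessage.
; It then spawns an explosion, destroys its mesh and collision, plays a hit sound and hides remaining visuals.
; A one-second delay precedes destroying the actor, after the trail is deactivated.
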(event Collision|EventActorBeginOverlap
  (params (OtherActor :type Actor%20Object%20Reference))
  (if (Utilities|DoesObjectImplementInterface OtherActor "/Script/flick_vr.IDamagable")
    (if (not (Actor|ActorHasTag OtherActor "Friendly"))
      (Class|IDamagable|AffectHealth(Message) OtherActor (Variables|Default|GetDamage))
      (Effects|SpawnEmitteratLocation "/Game/FlickerGame/Particles/P_misil_explosion.P_misil_explosion" (Transformation|GetWorldLocation (Variables|Default|GetDefaultSceneRoot)))
      (Components|DestroyComponent (Variables|Default|GetLaserMesh))
      (Audio|Components|Audio|Play (Variables|Default|Gethitsound) 0.0)
      (Rendering|SetVisibility (Variables|Default|GetScene) false true)
      (Components|Activation|Deactivate (Variables|Default|GetTrail))
      (Utilities|FlowControl|Delay 1.0)
      (Actor|DestroyActor))))

(fn ConstructionScript)