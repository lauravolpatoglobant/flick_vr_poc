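; Title screen actor for FlickerGame, with music and animated lighting that other code can show or hide.
; On BeginPlay it caches its location and starts a timeline that moves a point light to create a spinning effect.
; ShowScreen and HideScreen start or fade the music and restart separate timelines driving height, scale and backlight intensity.
; The hide timeline makes the whole actor invisible when finished.
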(event Custom|HideScreen
  (bind _initiallocation (Variables|Default|GetinitialLocation))
  (bind (_x _y _z) (Math|Vector|BreakVector _initiallocation))
  ;[1 1 1] hides game title screen
  (Audio|Components|Audio|FadeOut (Variables|Default|Getmusic) 0.5 0.0 :!class /Script/Engine.AudioComponent)
  (Utilities|FlowControl|Sequence
    (:then_0
      (bind (_direction _position _light_intensity) (Timeline|Timeline_1 Stop)
        (:Update
          (Transformation|SetRelativeLocation (Variables|Default|GetDefaultSceneRoot) (Math|Vector|MakeVector _x _y (+ (- _z 2e+01) (* _position 2e+01))) false false)
          (Transformation|SetRelativeScale3D (Variables|Default|GetScene) (Math|Conversions|ToVector(Float) (* _position 1.25)))
          (Rendering|Components|Light|SetIntensity (Variables|Default|GetBacklight1) (* _light_intensity 1e+03)))
        (:Finished
          (Rendering|SetVisibility (Variables|Default|GetDefaultSceneRoot) false true))))
    (:then_1
      (Rendering|SetVisibility (Variables|Default|GetDefaultSceneRoot) true true)
      (Timeline|Timeline_1 PlayFromStart))))

(event Custom|ShowScreen
  (bind _music (Variables|Default|Getmusic))
  (bind _initiallocation (Variables|Default|GetinitialLocation))
  (bind (_x _y _z) (Math|Vector|BreakVector _initiallocation))
  ;[1 1 1] shows title screen
  (if (Audio|Components|Audio|IsPlaying _music)
    _
    (else
      (Audio|Components|Audio|Play _music 0.0)))
  (Utilities|FlowControl|Sequence
    (:then_0
      (bind (_direction _position _light_intensity) (Timeline|Timeline_3 Stop)
        (:Update
          (Transformation|SetRelativeLocation (Variables|Default|GetDefaultSceneRoot) (Math|Vector|MakeVector _x _y (+ (- _z 2e+01) (* _position 2e+01))) false false)
          (Transformation|SetRelativeScale3D (Variables|Default|GetScene) (Math|Conversions|ToVector(Float) (* _position 1.25)))
          (Rendering|Components|Light|SetIntensity (Variables|Default|GetBacklight1) (* _light_intensity 1e+03)))))
    (:then_1
      (Rendering|SetVisibility (Variables|Default|GetDefaultSceneRoot) true true)
      (Timeline|Timeline_3 PlayFromStart))))

(event EventBeginPlay
  (Variables|Default|SetinitialLocation (Transformation|GetWorldLocation (Variables|Default|GetDefaultSceneRoot)))
  (Utilities|FlowControl|Sequence
    (:then_0
      ;[1 1 1] spinning light
      (bind _position (Timeline|Timeline_0 Play)
        (:Update
          (Transformation|SetRelativeLocation (Variables|Default|GetPointLight) (* _position "50.000000,25.000000, 0") false false))))))

(fn ConstructionScript)